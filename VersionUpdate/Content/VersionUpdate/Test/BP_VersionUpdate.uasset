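; Test actor that exercises the VersionUpdateSubsystem's hot-patch flow and reports each stage in a BPW_VersionUpdateTest widget or printed messages.
; BeginPlay binds the subsystem delegates and initializes it, which triggers a synchronous server check over internal HTTP.
; Callbacks show check results and download progress, then install downloaded files after a short delay.
; The custom manifest-download hook is empty, and its SubmitServerManifestJson call is unwired.
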(event `self.ReceiveBeginPlay`
  (`KismetSystemLibrary.PrintString` "测试  Hello" true true (struct :`R` 1.0 :`G` 0.67367 :`A` 1.0) 60.0)
  (add `VersionUpdateSubsystem.OnVersionUpdateInitialized` (subsystem `VersionUpdateSubsystem`) (delegate `OnVersionUpdateInitialized_Event`))
  (add `VersionUpdateSubsystem.OnServerManifestRequested` (subsystem `VersionUpdateSubsystem`) (delegate `OnServerManifestRequested_Event`))
  (add `VersionUpdateSubsystem.OnVersionCheckCompleted` (subsystem `VersionUpdateSubsystem`) (delegate `OnVersionCheckCompleted_Event`))
  (add `VersionUpdateSubsystem.OnVersionDownloadProgress` (subsystem `VersionUpdateSubsystem`) (delegate `OnVersionDownloadProgress_Event`))
  (add `VersionUpdateSubsystem.OnPatchFileDownloadCompleted` (subsystem `VersionUpdateSubsystem`) (delegate `OnPatchFileDownloadCompleted_Event`))
  (add `VersionUpdateSubsystem.OnVersionDownloadCompleted` (subsystem `VersionUpdateSubsystem`) (delegate `OnVersionDownloadCompleted_Event`))
  (add `VersionUpdateSubsystem.OnVersionInstallCompleted` (subsystem `VersionUpdateSubsystem`) (delegate `OnVersionInstallCompleted_Event`))
  (`|ExecutionSequence`
    (:`then_1`
      (bind _returnvalue (`|CreateWidget` "/VersionUpdate/VersionUpdate/Test/BPW_VersionUpdateTest.BPW_VersionUpdateTest_C"))
      (`UserWidget.AddToViewport` _returnvalue 0)
      (set `self.TestWidget` _returnvalue)
      (`VersionUpdateSubsystem.InitializeVersionUpdate` (subsystem `VersionUpdateSubsystem`) (`self.In Current Version`)))))

(event `OnVersionUpdateInitialized_Event`
  (params (CurrentVersion :type String))
  (`Widget.SetVisibility` (`/VersionUpdate/VersionUpdate/Test/BPW_VersionUpdateTest.floatwin` (`self.TestWidget`)) "Visible")
  (`VersionUpdateSubsystem.RequestServerVersionCheck` (subsystem `VersionUpdateSubsystem`) true true))

(event `OnServerManifestRequested_Event`
  (params (ManifestURL :type String))
  ;[1 1 1] 由RequestServerVersionCheck 广播，如果不用内置下载方式，在这个事件填自己的下载逻辑
)

(event `OnVersionDownloadCompleted_Event`
  (params (bSucceeded :type Boolean))
  (bind _texttip (`/VersionUpdate/VersionUpdate/Test/BPW_VersionUpdateTest.TextTip` (`self.TestWidget`)))
  (if bSucceeded
    (`TextBlock.SetText` _texttip "下载成功")
    (`KismetSystemLibrary.Delay` 5.0)
    (`VersionUpdateSubsystem.InstallDownloadedFiles` (subsystem `VersionUpdateSubsystem`))
    (else
      (`TextBlock.SetText` _texttip "下载失败"))))

(event `OnVersionCheckCompleted_Event`
  (params (Result :type "EServerVersionResponseType Enum" :default "VERSION_HOTUPDATE"))
  (bind _testwidget (`self.TestWidget`))
  (bind _testwidget_2 (`self.TestWidget`))
  (bind _testwidget_3 (`self.TestWidget`))
  (bind _testwidget_4 (`self.TestWidget`))
  (switch `EServerVersionResponseType` Result
    (:`VERSION_HOTUPDATE`
      (`Widget.SetVisibility` (`/VersionUpdate/VersionUpdate/Test/BPW_VersionUpdateTest.floatwin` _testwidget_4) "Visible")
      (`TextBlock.SetText` (`/VersionUpdate/VersionUpdate/Test/BPW_VersionUpdateTest.TextTip` _testwidget_4) "有热补丁"))
    (:`MAJORVERSION_UPDATE`
      (`Widget.SetVisibility` (`/VersionUpdate/VersionUpdate/Test/BPW_VersionUpdateTest.floatwin` _testwidget_2) "Visible")
      (`TextBlock.SetText` (`/VersionUpdate/VersionUpdate/Test/BPW_VersionUpdateTest.TextTip` _testwidget_2) "有大版本"))
    (:`VERSION_EQUAL`
      (`KismetSystemLibrary.PrintString` "版本相同"))
    (:`CONNECTION_ERROR`
      (`Widget.SetVisibility` (`/VersionUpdate/VersionUpdate/Test/BPW_VersionUpdateTest.floatwin` _testwidget_3) "Visible")
      (`TextBlock.SetText` (`/VersionUpdate/VersionUpdate/Test/BPW_VersionUpdateTest.TextTip` _testwidget_3) "网络错误!"))
    (:`INITIALIZATION_ERROR`
      (`Widget.SetVisibility` (`/VersionUpdate/VersionUpdate/Test/BPW_VersionUpdateTest.floatwin` _testwidget) "Visible")
      (`TextBlock.SetText` (`/VersionUpdate/VersionUpdate/Test/BPW_VersionUpdateTest.TextTip` _testwidget) "初始化错误!"))))

(event `OnVersionDownloadProgress_Event`
  (params (Percentage :type "Float (single-precision)") (FileName :type String) (TotalBytes :type Integer64) (BytesReceived :type Integer64))
  (bind _testwidget (`self.TestWidget`))
  (`Widget.SetVisibility` (`/VersionUpdate/VersionUpdate/Test/BPW_VersionUpdateTest.Progress` _testwidget) "Visible")
  (`ProgressBar.SetPercent` (`/VersionUpdate/VersionUpdate/Test/BPW_VersionUpdateTest.ProgressBar` _testwidget) Percentage)
  (`TextBlock.SetText` (`/VersionUpdate/VersionUpdate/Test/BPW_VersionUpdateTest.PakNameText` _testwidget) (`KismetTextLibrary.Conv_StringToText` FileName))
  (`TextBlock.SetText` (`/VersionUpdate/VersionUpdate/Test/BPW_VersionUpdateTest.DownloadSize` _testwidget) (`KismetTextLibrary.Conv_StringToText` (`KismetStringLibrary.Concat_StrStr` (`KismetStringLibrary.Conv_Int64ToString` TotalBytes) "/" (`KismetStringLibrary.Conv_Int64ToString` BytesReceived)))))

(event `OnPatchFileDownloadCompleted_Event`
  (params (FileName :type String) (bSucceeded :type Boolean))
  (if bSucceeded
    (`KismetSystemLibrary.PrintString` (`KismetStringLibrary.Concat_StrStr` FileName "已下载"))
    (else
      (`KismetSystemLibrary.PrintString` (`KismetStringLibrary.Concat_StrStr` FileName "下载失败")))))

(event `OnVersionInstallCompleted_Event`
  (params (bSucceeded :type Boolean))
  (bind _texttip (`/VersionUpdate/VersionUpdate/Test/BPW_VersionUpdateTest.TextTip` (`self.TestWidget`)))
  (if bSucceeded
    (`TextBlock.SetText` _texttip "安装成功！")
    (else
      (`TextBlock.SetText` _texttip "失败"))))

(fn `UserConstructionScript`)